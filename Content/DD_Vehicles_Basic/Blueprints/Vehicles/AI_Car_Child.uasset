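; AI car child Blueprint that steers a vehicle along the spline of its ActivePath.
; BeginPlay zeroes the throttle, and each PawnSensing See Pawn event refreshes steering from Getpath.
; Getpath projects 200 units along the nearest spline tangent, snaps that point back onto the spline, and maps the yaw difference toward it to a clamped steering input.
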(event OnSeePawn(PawnSensing)
  (params (Pawn :type Pawn%20Object%20Reference))
  (bind _returnvalue (CallFunction|Getpath))
  (Class|ChaosVehicleMovementComponent|SetSteeringInput (Variables|Default|GetVehicleMovementComponent) _returnvalue))

(event EventBeginPlay
  (Class|ChaosVehicleMovementComponent|SetThrottleInput (Variables|Default|GetVehicleMovementComponent) 0.0))

(fn ConstructionScript
  (|CallParentFunction))

(fn Getpath
  (bind _returnvalue (Transformation|GetActorLocation))
  (bind _activepath (Variables|Default|GetActivePath))
  (bind _spline (Variables|/Game/DD_Vehicles_Basic/Blueprints/Vehicles/path.path_C|GetSpline _activepath))
  (return (Math|Float|MapRangeClamped (.yaw (Math|Rotator|Delta(Rotator) (Math|Rotator|FindLookatRotation _returnvalue (Spline|FindLocationClosesttoWorldLocation _spline (+ (* (Math|Vector|Normalize (Class|SplineComponent|FindTangentClosesttoWorldLocation _spline _returnvalue "World")) 2e+02) _returnvalue) "World")) (Transformation|GetActorRotation))) -9e+01 9e+01 -1.0 1.0)))